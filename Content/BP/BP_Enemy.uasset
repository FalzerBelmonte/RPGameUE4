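; BP_Enemy is a character that players can talk to through a dialogue widget when nearby.
; Box2 overlaps with INT_Player actors tilt its two brows, create WBP_Dialogue for the local player, and undo both on exit.
; Interact notifies that widget, then fills in the face texture, name, first text line and an exclamation-mark emoticon.
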(event `/Game/BP/Interface/INT_Interact.Interact`
  (bind _dialogue (`self.Dialogue`))
  (`/Engine/EditorBlueprintResources/StandardMacros.IsValid` _dialogue
    (:`Is Valid`
      (`/Game/Widgets/WBP_Dialogue.InteractHappen` _dialogue)
      (`|ExecutionSequence`
        (:`then_0`
          (bind _output_get (set `self.Dialogue` _dialogue))
          (`Border.SetBrushFromTexture` (`/Game/Widgets/WBP_Dialogue.CharacterFaces` _output_get) "/Game/PugsiUwu/Assets/Faces/Face.Face")
          (set `/Game/Widgets/WBP_Dialogue.Dialog` (`|GetArrayItem` (`self.MyText`)) _output_get)
          (set `/Game/Widgets/WBP_Dialogue.NPCName` (`self.Name`) _output_get))
        (:`then_1`
          (bind _output_get_2 (set `self.Dialogue` _dialogue))
          (`Border.SetBrushFromTexture` (`/Game/Widgets/WBP_Dialogue.Emoticon` _output_get_2) "/Game/PugsiUwu/Assets/Icons/ExclamationMark.ExclamationMark"))))))

(event `self.Box2.OnComponentBeginOverlap`
  (params (OverlappedComponent :type "PrimitiveComponent Object Reference") (OtherActor :type "Actor Object Reference") (OtherComp :type "PrimitiveComponent Object Reference") (OtherBodyIndex :type Integer) (bFromSweep :type Boolean) (SweepResult :type "HitResult Structure (by ref)"))
  (bind _returnvalue (`self.GetInstigatorController` OtherActor))
  (if (`KismetSystemLibrary.DoesImplementInterface` OtherActor "/Game/BP/Interface/INT_Player.INT_Player_C")
    (`|ExecutionSequence`
      (:`then_0`
        (`SceneComponent.K2_AddLocalRotation` (`self.Brow`) (* (`KismetMathLibrary.MakeRotator` 0.0 20.0) 1.0) false false))
      (:`then_1`
        (`SceneComponent.K2_AddLocalRotation` (`self.Brow2`) (* (`KismetMathLibrary.MakeRotator` 0.0 -20.0) 1.0) false false))
      (:`then_2`
        (`/Engine/EditorBlueprintResources/StandardMacros.IsValid` (`self.Dialogue`)
          (:`Is Not Valid`
            (`/Engine/EditorBlueprintResources/StandardMacros.IsValid` _returnvalue
              (:`Is Valid`
                (if (`Controller.IsLocalPlayerController` _returnvalue)
                  (bind _returnvalue_2 (`|CreateWidget` "/Game/Widgets/WBP_Dialogue.WBP_Dialogue_C"))
                  (bind _output_get (set `self.Dialogue` _returnvalue_2))
                  (`/Game/Widgets/WBP_Dialogue.WhenInteract` _output_get)
                  (`UserWidget.AddToViewport` _returnvalue_2 1)
                  (`UserWidget.AddToViewport` _returnvalue_2 1))))))))))

(event `self.Box2.OnComponentEndOverlap`
  (params (OverlappedComponent :type "PrimitiveComponent Object Reference") (OtherActor :type "Actor Object Reference") (OtherComp :type "PrimitiveComponent Object Reference") (OtherBodyIndex :type Integer))
  (bind _dialogue (`self.Dialogue`))
  (if (`KismetSystemLibrary.DoesImplementInterface` OtherActor "/Game/BP/Interface/INT_Player.INT_Player_C")
    (`|ExecutionSequence`
      (:`then_0`
        (`SceneComponent.K2_AddLocalRotation` (`self.Brow`) (* (`KismetMathLibrary.MakeRotator` 0.0 -20.0) 1.0) false false))
      (:`then_1`
        (`SceneComponent.K2_AddLocalRotation` (`self.Brow2`) (* (`KismetMathLibrary.MakeRotator` 0.0 20.0) 1.0) false false))
      (:`then_2`
        (`/Engine/EditorBlueprintResources/StandardMacros.IsValid` OtherActor
          (:`Is Valid`
            (if true
              (`/Engine/EditorBlueprintResources/StandardMacros.IsValid` _dialogue
                (:`Is Valid`
                  (`Widget.RemoveFromParent` _dialogue)
                  (set `self.Dialogue` null))))))))))

(fn `UserConstructionScript`)
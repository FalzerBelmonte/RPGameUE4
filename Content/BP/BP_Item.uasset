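; BP_Item is a world pickup that displays a shiny particle effect until the player collects it.
; Its box overlap checks for INT_Player, creating a WBP_ItemFound prompt when the player is near and removing it on exit.
; Interact works only while that widget exists: it switches it to picked-up state with the first name and description entries, then after a short delay removes widget, effect and actor.
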(event `self.ReceiveBeginPlay`
  (bind _returnvalue (`NiagaraFunctionLibrary.SpawnSystemAtLocation` "/Game/Assets/Nigara/Item/Item_Emitter_System.Item_Emitter_System" (`SceneComponent.K2_GetComponentLocation` (`self.DefaultSceneRoot`))))
  (set `self.Shiny` _returnvalue))

(event `/Game/BP/Interface/INT_Interact.Interact`
  (bind _itempick (`self.ItemPick`))
  (`/Engine/EditorBlueprintResources/StandardMacros.IsValid` _itempick
    (:`Is Valid`
      (`/Game/Widgets/WBP_ItemFound.PickedUp` _itempick)
      (set `/Game/Widgets/WBP_ItemFound.ItemDescription` (`|GetArrayItem` (`self.Description`)) _itempick)
      (set `/Game/Widgets/WBP_ItemFound.ItemName` (`|GetArrayItem` (`self.ItemName`)) _itempick)
      (`KismetSystemLibrary.Delay` 2.0)
      (`Widget.RemoveFromParent` _itempick)
      (set `self.ItemPick` null)
      (`ActorComponent.K2_DestroyComponent` (`self.Shiny`))
      (`self.K2_DestroyActor`))))

(event `self.Box.OnComponentBeginOverlap`
  (params (OverlappedComponent :type "PrimitiveComponent Object Reference") (OtherActor :type "Actor Object Reference") (OtherComp :type "PrimitiveComponent Object Reference") (OtherBodyIndex :type Integer) (bFromSweep :type Boolean) (SweepResult :type "HitResult Structure (by ref)"))
  (if (`KismetSystemLibrary.DoesImplementInterface` OtherActor "/Game/BP/Interface/INT_Player.INT_Player_C")
    (bind _returnvalue (`|CreateWidget` "/Game/Widgets/WBP_ItemFound.WBP_ItemFound_C"))
    (bind _output_get (set `self.ItemPick` _returnvalue))
    (`/Game/Widgets/WBP_ItemFound.PlayerNear` _output_get)
    (`UserWidget.AddToViewport` _output_get 0)))

(event `self.Box.OnComponentEndOverlap`
  (params (OverlappedComponent :type "PrimitiveComponent Object Reference") (OtherActor :type "Actor Object Reference") (OtherComp :type "PrimitiveComponent Object Reference") (OtherBodyIndex :type Integer))
  (bind _itempick (`self.ItemPick`))
  (if (`KismetSystemLibrary.DoesImplementInterface` OtherActor "/Game/BP/Interface/INT_Player.INT_Player_C")
    (`/Engine/EditorBlueprintResources/StandardMacros.IsValid` OtherActor
      (:`Is Valid`
        (if true
          (`/Engine/EditorBlueprintResources/StandardMacros.IsValid` _itempick
            (:`Is Valid`
              (`Widget.RemoveFromParent` _itempick)
              (set `self.ItemPick` null))))))))

(fn `UserConstructionScript`)
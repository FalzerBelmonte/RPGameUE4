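; A consumable example item for the RPG Development Kit inventory system that launches its owner upward.
; On the inventory use-item interface event it casts the item's owning actor to Character, launches it straight up by adding vertical velocity, then destroys itself.
; If the owner is not a Character, it only prints a failure message.
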(event `/Game/BhandanaDesign/RPG_DevelopmentKit/InventorySystem/Interfaces/BPI_InventorySystem.BPI_INV_Use Item`
  (bind _ascharacter (cast `Character` (`self.ItemOwnerActor`))
    (:`then`
      (`Character.LaunchCharacter` _ascharacter (0.0 0.0 500.0) false false)
      (`self.K2_DestroyActor`))
    (:`CastFailed`
      (`KismetSystemLibrary.PrintString` "Failed"))))

(fn `UserConstructionScript`
  (`parent.UserConstructionScript`))
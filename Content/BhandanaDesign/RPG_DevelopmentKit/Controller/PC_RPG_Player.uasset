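; Player controller for the RPG kit that owns the player's inventory and handles menu input.
; The Inventory input toggles an inventory window, optionally disabling pawn input, while holding Left Alt shows the cursor.
; It implements inventory interface calls to add, remove and retrieve items.
; Adding stacks matching items of any type except Equipment; removing decrements the slot's quantity or removes the entry when it reaches zero.
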(event `Key|LeftAlt`
  (params (Key :type "Key Structure"))
  (:`Pressed`
    (`WidgetBlueprintLibrary.SetInputMode_GameAndUIEx` self null)
    (set `self.bShowMouseCursor` true))
  (:`Released`
    (`WidgetBlueprintLibrary.SetInputMode_GameOnly` self)
    (set `self.bShowMouseCursor` false)))

(event `self.ReceivePossess`
  (params (PossessedPawn :type "Pawn Object Reference"))
  (set `self.MyPawn` PossessedPawn))

(event `InputAction|Inventory`
  (params (Key :type "Key Structure"))
  (:`Pressed`
    (`/Engine/EditorBlueprintResources/StandardMacros.FlipFlop`
      (:`A`
        (if (not (`self.CanWalkInMenu`))
          (`self.DisableInput` (`self.MyPawn`) null))
        (bind _returnvalue (`|CreateWidget` "/Game/BhandanaDesign/RPG_DevelopmentKit/InventorySystem/UI_Widgets/WBP_InventoryWindow.WBP_InventoryWindow_C" self))
        (`UserWidget.AddToViewport` _returnvalue 0)
        (`WidgetBlueprintLibrary.SetInputMode_GameAndUIEx` self _returnvalue)
        (set `self.bShowMouseCursor` true))
      (:`B`
        (`self.EnableInput` (`self.MyPawn`) null)
        (`Widget.RemoveFromParent` _returnvalue)
        (`WidgetBlueprintLibrary.SetInputMode_GameOnly` self)
        (set `self.bShowMouseCursor` false)))))

(event `/Game/BhandanaDesign/RPG_DevelopmentKit/InventorySystem/Interfaces/BPI_InventorySystem.BPI_INV_AddItem`
  (params (`Item to Add` :type "/Game/BhandanaDesign/RPG_DevelopmentKit/InventorySystem/Structures/ST_Item Structure"))
  (bind (_name _rarity _itemtype) (break `/Game/BhandanaDesign/RPG_DevelopmentKit/InventorySystem/Structures/ST_Item` `Item to Add`))
  (set `self.IsItemLoop` false)
  (for (_array_element _array_index) (`self.Inventory`)
    (bind (_name_2 _rarity_2 _itemtype_2 _itemactor _description _quantitiy) (break `/Game/BhandanaDesign/RPG_DevelopmentKit/InventorySystem/Structures/ST_Item` _array_element))
    (if (and (== _name _name_2) (== _itemtype _itemtype_2) (select `/Game/BhandanaDesign/RPG_DevelopmentKit/InventorySystem/Enumerators/ENUM_ItemTypes` _itemtype_2 :`NewEnumerator0` true :`NewEnumerator2` true :`NewEnumerator3` true))
      (set `self.IsItemLoop` true)
      (break)))
  (if (`self.IsItemLoop`)
    (bind _structout (setmembers `/Game/BhandanaDesign/RPG_DevelopmentKit/InventorySystem/Structures/ST_Item` :`StructRef` _array_element :`Quantitiy` (+ _quantitiy (`.Quantitiy_25_D0B037E143DE9F427B54F598D9AD63ED` (break `/Game/BhandanaDesign/RPG_DevelopmentKit/InventorySystem/Structures/ST_Item` `Item to Add`)))))
    (`KismetArrayLibrary.Array_Set` (`self.Inventory`) _array_index _structout)
    (else
      (`KismetArrayLibrary.Array_Add` (`self.Inventory`) `Item to Add`))))

(fn `BPI_INV_RemoveItem`
  (params (Item :type "/Game/BhandanaDesign/RPG_DevelopmentKit/InventorySystem/Structures/ST_Item Structure") (`Number to Remove` :type Integer) (ItemSlot :type Integer))
  (returns (`is Gone` :type Boolean))
  (bind _output (`|GetArrayItem` (`self.Inventory`) ItemSlot))
  (bind _returnvalue (- (`.Quantitiy_25_D0B037E143DE9F427B54F598D9AD63ED` (break `/Game/BhandanaDesign/RPG_DevelopmentKit/InventorySystem/Structures/ST_Item` _output)) `Number to Remove`))
  (if (<= _returnvalue 0)
    (`KismetArrayLibrary.Array_RemoveItem` (`self.Inventory`) _output)
    (return true)
    (else
      (bind _structout (setmembers `/Game/BhandanaDesign/RPG_DevelopmentKit/InventorySystem/Structures/ST_Item` :`StructRef` _output :`Quantitiy` _returnvalue))
      (`KismetArrayLibrary.Array_Set` (`self.Inventory`) ItemSlot _structout)
      (return false))))

(fn `BPI_INV_Retrieve Inventory`
  (returns (Inventory :type "Array of /Game/BhandanaDesign/RPG_DevelopmentKit/InventorySystem/Structures/ST_Item Structure"))
  (return (`self.Inventory`)))

(fn `UserConstructionScript`)